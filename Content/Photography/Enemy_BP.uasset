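; Placeholder wandering character for a photography game, intended as a subject whose state can later feed photo scoring.
; It loops between picking a random navigable point, moving there with AIMoveTo at randomly full or half speed, and pausing for a random delay.
; GetState derives an enum from velocity and speed cap, distinguishing stationary, slow and full-speed movement.
; The construction script tints the body through a dynamic material instance.
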(event `self.ReceiveBeginPlay`
  ;[1 0.00687 0] Placeholder: Basic wandering logic.
  ; TODO: replace with blackboard system
  ; TODO: add system for recording the "state" of the character for scoring purposes
  ; TODO: consider adding components that allow for scoring of individual parts (e.g. Face = bonus points)
  (set `self.DefaultWalkSpeed` (`CharacterMovementComponent.MaxWalkSpeed` (`self.CharacterMovement`)))
  (`self.GetNewLocation` :!label _label)
  (`self.GoToLocation`))

(event `GoToLocation`
  ;[1 0.00687 0] Placeholder: Basic wandering logic.
  ; TODO: replace with blackboard system
  ; TODO: add system for recording the "state" of the character for scoring purposes
  ; TODO: consider adding components that allow for scoring of individual parts (e.g. Face = bonus points)
  (`|AIMoveTo` self (`self.WanderLocation`) null
    (:`OnSuccess`
      _)
    (:`OnFail`
      _))
  (`KismetSystemLibrary.Delay` (`KismetMathLibrary.RandomFloatInRange` 1.0 10.0))
  (goto _label))

(event `GetNewLocation`
  (bind _defaultwalkspeed (`self.DefaultWalkSpeed`))
  (bind _charactermovement (`self.CharacterMovement`))
  ;[1 0.00687 0] Placeholder: Basic wandering logic.
  ; TODO: replace with blackboard system
  ; TODO: add system for recording the "state" of the character for scoring purposes
  ; TODO: consider adding components that allow for scoring of individual parts (e.g. Face = bonus points)
  (bind _randomlocation (`NavigationSystemV1.K2_GetRandomLocationInNavigableRadius` (`self.K2_GetActorLocation`) (`self.WanderRadius`) null null))
  (set `self.WanderLocation` _randomlocation)
  (`/Engine/EditorBlueprintResources/StandardMacros.CompareFloat` (`KismetMathLibrary.RandomFloat`) 0.5
    (:`>`
      (set `CharacterMovementComponent.MaxWalkSpeed` _defaultwalkspeed _charactermovement :!label _label_2))
    (:`==`
      (goto _label_2))
    (:`<`
      (set `CharacterMovementComponent.MaxWalkSpeed` (/ _defaultwalkspeed 2.0) _charactermovement))))

(fn `Get State`
  (returns (NewParam :type "/Game/Photography/TargetState Enum"))
  (bind _charactermovement (`self.CharacterMovement`))
  (if (== (`KismetMathLibrary.VSize` (`CharacterMovementComponent.GetLastUpdateVelocity` _charactermovement)) 0.0)
    (return "NewEnumerator0")
    (else
      (`/Engine/EditorBlueprintResources/StandardMacros.CompareFloat` (`CharacterMovementComponent.MaxWalkSpeed` _charactermovement) (`self.DefaultWalkSpeed`)
        (:`>`
          _)
        (:`==`
          _)
        (:`<`
          (return "NewEnumerator1")))
      (return "NewEnumerator2"))))

(fn `UserConstructionScript`
  (bind _returnvalue (`PrimitiveComponent.CreateDynamicMaterialInstance` (`self.Mesh`) 0 "/Game/Mannequin/Character/Materials/M_UE4Man_Body.M_UE4Man_Body" "None"))
  (`MaterialInstanceDynamic.SetVectorParameterValue` _returnvalue "BodyColor" (`self.BodyColour`)))